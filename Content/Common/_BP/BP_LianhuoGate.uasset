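; BP_LianhuoGate is a one-shot gate trigger that brings in the BP_Lianhuo AI enemy.
; When BP_Saiqi overlaps it and no BP_Lianhuo exists, the MoveUp timeline offsets the mesh along local Z.
; A five-second Delay hanging off the timeline's Update then spawns BP_Lianhuo with its behavior tree at a fixed offset from the mesh and destroys the gate.
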(event `self.ReceiveActorBeginOverlap`
  (params (OtherActor :type "Actor Object Reference"))
  (bind _outactors (`GameplayStatics.GetAllActorsOfClass` "/Game/Common/_BP/Character/Enemy/Boss/Lianhuo/BP_Lianhuo.BP_Lianhuo_C"))
  (if (== (`KismetArrayLibrary.Array_Length` _outactors) 0)
    (cast `/Game/Common/_BP/Character/Player/Saiqi/BP_Saiqi` OtherActor)
    (bind (_direction `_새_트랙_0`) (`Timeline|MoveUp` :!via `PlayFromStart`)
      (:`Update`
        (`SceneComponent.K2_AddLocalOffset` (`self.StaticMesh`) (`KismetMathLibrary.MakeVector` 0.0 0.0 (* `_새_트랙_0` 2.0)) false false)
        (`KismetSystemLibrary.Delay` 5.0)
        (`AIBlueprintHelperLibrary.SpawnAIFromClass` "/Game/Common/_BP/Character/Enemy/Boss/Lianhuo/BP_Lianhuo.BP_Lianhuo_C" "/Game/Common/_BP/Character/Enemy/Boss/Lianhuo/AI/BT_Enemy_Lianhuo.BT_Enemy_Lianhuo" (+ (`SceneComponent.K2_GetComponentLocation` (`self.StaticMesh`)) (0.0 -3500.0 0.0)) (struct :`Yaw` 90.0) false null)
        (`self.K2_DestroyActor`)))))

(fn `UserConstructionScript`)