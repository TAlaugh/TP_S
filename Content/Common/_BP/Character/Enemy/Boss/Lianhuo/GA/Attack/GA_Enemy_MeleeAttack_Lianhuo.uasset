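; Melee attack gameplay ability for the Lianhuo boss enemy, which plays an attack montage and deals damage on hit.
; While the montage plays, it listens for melee hit events and applies a damage effect spec to each event's target.
; A successful application sends a HitReact event to the target; the weapon hit sound cue node is left unconnected.
; The ability ends when the montage completes, blends out, is interrupted or is cancelled.
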(event `self.K2_ActivateAbility`
  (`AbilityTask_PlayMontageAndWait.CreatePlayMontageAndWaitProxy` "None" (`self.Montage to Play`)
    (:`then`
      (bind (_asynctaskproxy _payload) (`AbilityTask_WaitGameplayEvent.WaitGameplayEvent` (struct :`TagName` "Shared.Event.Hit.Melee") null)
        (:`EventReceived`
          (`self.HandleApplyDamage` _payload))))
    (:`OnCompleted`
      (`self.K2_EndAbility` :!label _label))
    (:`OnBlendOut`
      (goto _label))
    (:`OnInterrupted`
      (goto _label))
    (:`OnCancelled`
      (goto _label))))

(fn `HandleApplyDamage`
  (params (InPayload :type "GameplayEventData Structure"))
  (bind (_eventtag _instigator _target) (break `GameplayEventData` InPayload))
  (`self.BP_ApplyEffectSpecHandleToTarget` _target (`self.MakeEnemyDamageEffectSpecHandle` "/Game/Common/_BP/Character/Enemy/Shared/GE/GE_DealDamage.GE_DealDamage_C" (`self.Damage Float`))
    (:`Successful`
      (`|ExecutionSequence`
        (:`then_1`
          ;[1 1 1] 피격자(플레이어)에게 HitReact태그를 주입 및 사운드 실행
          (`AbilitySystemBlueprintLibrary.SendGameplayEventToActor` _target (struct :`TagName` "Shared.Event.HitReact") (`local.InPayload`)))))))