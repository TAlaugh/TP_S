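; Melee attack ability for the Lianhuo boss's first attack, adding a slash projectile while rage is active.
; WhileRageActive waits for the SpawnProjectile gameplay event, then spawns BP_EnemyProjectile_Slash at the equipped weapon's RageSlashSocket with a GE_DealDamage spec.
; The projectile takes its roll from the socket and yaw from the boss's forward vector.
; Activate and end overrides are disabled stubs.
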(event `self.WhileRageActive`
  (bind _returnvalue (`self.GetEnemyCharacterFromActorInfo`))
  (bind (_returnvalue_roll _returnvalue_pitch _returnvalue_yaw) (`KismetMathLibrary.BreakRotator` (`KismetMathLibrary.MakeRotFromX` (`Actor.GetActorForwardVector` _returnvalue))))
  (bind _returnvalue_2 (`SceneComponent.GetSocketTransform` (`BaseWeapon.WeaponMesh` (`EnemyCombatComponent.GetCharacterCurrentEquippedWeapon` (`self.GetEnemyCombatComponentFromActorInfo`))) "RageSlashSocket" "RTS_World"))
  (`AbilityTask_WaitGameplayEvent.WaitGameplayEvent` (struct :`TagName` "Shared.Event.SpawnProjectile") null
    (:`EventReceived`
      (`|SpawnActorFromClass` "/Game/Common/_BP/Character/Enemy/Boss/Lianhuo/BP_EnemyProjectile_Slash.BP_EnemyProjectile_Slash_C" (`KismetMathLibrary.MakeTransform` (.location _returnvalue_2) (`KismetMathLibrary.MakeRotator` (.roll (.rotation _returnvalue_2)) 0.0 _returnvalue_yaw)) "AdjustIfPossibleButAlwaysSpawn" "MultiplyWithRoot" null (`self.MakeEnemyDamageEffectSpecHandle` "/Script/TP_S.GE_DealDamage" (`self.Damage Float`)) _returnvalue))))