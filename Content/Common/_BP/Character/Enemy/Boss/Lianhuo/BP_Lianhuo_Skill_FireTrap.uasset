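; Fire trap actor for the Lianhuo boss's skill, a delayed ground explosion that knocks BP_Saiqi into the air.
; After a short telegraph delay it spawns the explosion Niagara effect and turns on overlap events on its Box, then destroys itself half a second later.
; An overlapping BP_Saiqi receives a strong upward impulse through CharacterMovement; the graph applies no damage.
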(event `self.ReceiveBeginPlay`
  (`KismetSystemLibrary.Delay` 2.5)
  (`NiagaraFunctionLibrary.SpawnSystemAtLocation` "/Game/HeavyAssets/NS/_InUse/NS_ExplosionGround_FireTrap.NS_ExplosionGround_FireTrap" (`self.K2_GetActorLocation`))
  (set `PrimitiveComponent.bGenerateOverlapEvents` true (`self.Box`))
  (`KismetSystemLibrary.Delay` 0.5)
  (`self.K2_DestroyActor` self))

(event `self.ReceiveActorBeginOverlap`
  (params (OtherActor :type "Actor Object Reference"))
  (bind _asbp_saiqi (cast `/Game/Common/_BP/Character/Player/Saiqi/BP_Saiqi` OtherActor))
  (`CharacterMovementComponent.AddImpulse` (`Character.CharacterMovement` _asbp_saiqi) (0.0 0.0 20000.0) false))

(fn `UserConstructionScript`)