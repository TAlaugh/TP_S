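; Base enemy character Blueprint that handles spawn and death presentation for enemies.
; On BeginPlay, a timeline animates the DissolveAmount material parameter on the body and equipped weapon while a random spawn montage plays, if any exist.
; On death, it pauses animation, disables capsule collision, removes enemy UI widgets and runs a second dissolve timeline.
; Both timelines derive their play rate from configurable total durations.
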(event `self.ReceiveBeginPlay`
  (bind _spawnmontage (`self.SpawnMontage`))
  (bind _returnvalue (`EnemyCombatComponent.GetCharacterCurrentEquippedWeapon` (`self.EnemyCombatComponent`)))
  (`|ExecutionSequence`
    (:`then_0`
      (`TimelineComponent.SetPlayRate` (`self.EntryRestoreTimeline`) (/ 1.0 (`self.TotalEntryRestoreTime`)))
      (bind (_direction _dissovetime) (`Timeline|EntryRestoreTimeline` :!via `PlayFromStart`)
        (:`Update`
          (`MeshComponent.SetScalarParameterValueOnMaterials` (`self.Mesh`) "DissolveAmount" _dissovetime)
          (`/Engine/EditorBlueprintResources/StandardMacros.IsValid` _returnvalue
            (:`Is Valid`
              (`MeshComponent.SetScalarParameterValueOnMaterials` (`BaseWeapon.WeaponMesh` _returnvalue) "DissolveAmount" _dissovetime))))))
    (:`then_1`
      (if (`KismetArrayLibrary.Array_IsNotEmpty` _spawnmontage)
        (`self.PlayAnimMontage` (`KismetArrayLibrary.Array_Random` _spawnmontage))))))

(event `/Game/Common/_BP/Character/Enemy/Shared/BPI_EnemyDead.OnEnemyDead`
  (bind _returnvalue (`EnemyCombatComponent.GetCharacterCurrentEquippedWeapon` (`self.EnemyCombatComponent`)))
  (`|ExecutionSequence`
    (:`then_0`
      (set `SkeletalMeshComponent.bPauseAnims` true (`self.Mesh`))
      (`PrimitiveComponent.SetCollisionEnabled` (`self.CapsuleComponent`) "NoCollision"))
    (:`then_1`
      (`BaseUIComponent.RemoveEnemyDrawnWidgetIfAny` (`self.EnemyUIComponent`)))
    (:`then_2`
      (`TimelineComponent.SetPlayRate` (`self.Dissolve Timeline`) (/ 1.0 (`self.TotalDissolveTime`)))
      (bind (_direction _dissovetime) (`Timeline|Dissolve Timeline` :!via `PlayFromStart`)
        (:`Update`
          (`MeshComponent.SetScalarParameterValueOnMaterials` (`self.Mesh`) "DissolveAmount" _dissovetime)
          (`/Engine/EditorBlueprintResources/StandardMacros.IsValid` _returnvalue
            (:`Is Valid`
              (`MeshComponent.SetScalarParameterValueOnMaterials` (`BaseWeapon.WeaponMesh` _returnvalue) "DissolveAmount" _dissovetime))))))))

(fn `UserConstructionScript`)