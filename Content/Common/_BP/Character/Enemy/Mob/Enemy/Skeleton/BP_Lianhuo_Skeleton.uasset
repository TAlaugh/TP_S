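; Skeleton enemy character blueprint that handles the dissolve effects for entering and leaving play.
; BeginPlay animates DissolveAmount on the body and equipped weapon materials while playing a random entry montage.
; A custom event freezes animation, disables capsule collision, clears enemy UI widgets and runs the exit dissolve, destroying weapon and actor when the weapon mesh is valid.
; Both timelines scale play rate by configurable durations.
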(event `self.ReceiveBeginPlay`
  (bind _entrymontagetoplay (`self.EntryMontageToPlay`))
  (bind _returnvalue (`EnemyCombatComponent.GetCharacterCurrentEquippedWeapon` (`self.EnemyCombatComponent`)))
  (`|ExecutionSequence`
    (:`then_0`
      (`TimelineComponent.SetPlayRate` (`self.타임라인_0`) (/ 1.0 (`self.TotalEntryRestoreTime`)))
      (bind (_direction `_새_트랙_1`) (`Timeline|타임라인_0` :!via `PlayFromStart`)
        (:`Update`
          (`MeshComponent.SetScalarParameterValueOnMaterials` (`self.Mesh`) "DissolveAmount" `_새_트랙_1`)
          (`/Engine/EditorBlueprintResources/StandardMacros.IsValid` _returnvalue
            (:`Is Valid`
              (`MeshComponent.SetScalarParameterValueOnMaterials` (`BaseWeapon.WeaponMesh` _returnvalue) "DissolveAmount" `_새_트랙_1`))))))
    (:`then_1`
      (if (`KismetArrayLibrary.Array_IsNotEmpty` _entrymontagetoplay)
        (`self.PlayAnimMontage` (`KismetArrayLibrary.Array_Random` _entrymontagetoplay))))))

(event `CustomEvent`
  (bind _returnvalue (`EnemyCombatComponent.GetCharacterCurrentEquippedWeapon` (`self.EnemyCombatComponent`)))
  (`|ExecutionSequence`
    (:`then_0`
      (set `SkeletalMeshComponent.bPauseAnims` true (`self.Mesh`))
      (`PrimitiveComponent.SetCollisionEnabled` (`self.CapsuleComponent`) "NoCollision"))
    (:`then_1`
      (`BaseUIComponent.RemoveEnemyDrawnWidgetIfAny` (`self.EnemyUIComponent`)))
    (:`then_2`
      (`TimelineComponent.SetPlayRate` (`self.타임라인`) (/ 1.0 (`self.DissolveTime`)))
      (bind (_direction `_새_트랙_0`) (`Timeline|타임라인` :!via `PlayFromStart`)
        (:`Update`
          (`MeshComponent.SetScalarParameterValueOnMaterials` (`self.Mesh`) "DissolveAmount" `_새_트랙_0`)
          (`MeshComponent.SetScalarParameterValueOnMaterials` (`BaseWeapon.WeaponMesh` (`EnemyCombatComponent.GetCharacterCurrentEquippedWeapon` (`self.EnemyCombatComponent`))) "DissolveAmount" `_새_트랙_0`))
        (:`Finished`
          (`/Engine/EditorBlueprintResources/StandardMacros.IsValid` (`BaseWeapon.WeaponMesh` _returnvalue)
            (:`Is Valid`
              (`self.K2_DestroyActor` _returnvalue)
              (`self.K2_DestroyActor`))))))))

(fn `UserConstructionScript`)