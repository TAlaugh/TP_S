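; Game mode Blueprint for the Boss06 stage that presents wave-based enemy spawning progress to the player.
; Stage trigger activation binds a handler to game mode state changes, which creates countdown or plain text widgets for incoming, current and completed waves.
; On the final wave it zeroes the enemy spawn delay and shows a delayed "Last Wave" banner.
; Win and player death only print debug strings.
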(event `self.ReceiveBeginPlay`)

(event `self.OnStageTriggerActivated`
  (add `self.OnBoss06GameModeStateChanged` (delegate `OnBoss06GameModeStateChanged_Event`)))

(event `OnBoss06GameModeStateChanged_Event` :!signature `self.OnBoss06GameModeStateChanged`
  (params (CurrentState :type "EBoss06GameModeState Enum" :default "WaitSpawnNewWave"))
  (switch `EBoss06GameModeState` CurrentState
    (:`WaitSpawnNewWave`
      (`self.CreateWaveWidgetCountDown` "Wave Is Comming" (`self.SpawnNewWaveWaitTime`)))
    (:`SpawnNewWave`
      (`self.Create Wave Widget No Count Down` (`|FormatText` "Wave{CurrentWaveCount}" (`self.CurrentWaveCount`)))
      (if (== (`self.CurrentWaveCount`) (`self.TotalWavesToSpawn`))
        (set `self.SpawnEnemiesDelayTime` 0.0)
        (`KismetSystemLibrary.Delay` 2.0)
        (`self.Create Wave Widget No Count Down` "Last Wave")))
    (:`WaveComplete`
      (`self.CreateWaveWidgetCountDown` (`|FormatText` "Wave{CurrentWaveCount} completed" (`self.CurrentWaveCount`)) (`self.WaveCompletedWaitTime`)))
    (:`AllWavesDone`
      (`KismetSystemLibrary.PrintString` "win" true true (struct :`G` 0.66 :`B` 1.0 :`A` 1.0) 5.0))
    (:`PlayerDied`
      (`KismetSystemLibrary.PrintString` "PlayerDied" true true (struct :`G` 0.66 :`B` 1.0 :`A` 1.0) 5.0))))

(fn `Create Wave Widget No Count Down`
  (params (TextContextToDisplay :type Text))
  (bind _returnvalue (`|CreateWidget` "/Game/Common/_BP/Character/Enemy/Boss/Boss_06/Widget/WBP_WaveTextNoCountDown.WBP_WaveTextNoCountDown_C"))
  (`UserWidget.AddToViewport` _returnvalue 0)
  (`TextBlock.SetText` (`/Game/Common/_BP/Character/Enemy/Boss/Boss_06/Widget/WBP_WaveTextNoCountDown.TextBlock_WaveText` _returnvalue) (`local.TextContextToDisplay`)))

(fn `CreateWaveWidgetCountDown`
  (params (TextToContentDisplay :type Text) (InTotalCountDownTime :type "Float (double-precision)"))
  (bind _returnvalue (`|CreateWidget` "/Game/Common/_BP/Character/Enemy/Boss/Boss_06/Widget/WBP_WaveTextWithCountDown.WBP_WaveTextWithCountDown_C"))
  (`UserWidget.AddToViewport` _returnvalue 0)
  (`TextBlock.SetText` (`/Game/Common/_BP/Character/Enemy/Boss/Boss_06/Widget/WBP_WaveTextWithCountDown.TextBlock_WaveText` _returnvalue) (`local.TextToContentDisplay`))
  (`/Game/Common/_BP/Character/Enemy/Boss/Boss_06/Widget/WBP_WaveTextWithCountDown.StartCountDown` _returnvalue (`local.InTotalCountDownTime`)))

(fn `UserConstructionScript`)