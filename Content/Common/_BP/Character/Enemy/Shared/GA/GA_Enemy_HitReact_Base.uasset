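; Base enemy hit-react gameplay ability, activated by a gameplay event, that plays the reaction to being hit.
; With a montage, it turns the enemy toward the event instigator and plays a random hit-react montage until it ends.
; Without one, it ends after a short delay.
; Both paths apply an under-attack effect to the owner and toggle a hit-flash material parameter, which is reset when the ability ends.
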(event `self.K2_ActivateAbilityFromEvent`
  (params (EventData :type "GameplayEventData Structure (by ref)"))
  (`|ExecutionSequence`
    (:`then_0`
      (if (`self.HasMontage`)
        (`Actor.K2_SetActorRotation` (`self.GetEnemyCharacterFromActorInfo`) (`KismetMathLibrary.FindLookAtRotation` (`Actor.K2_GetActorLocation` (`self.GetEnemyCharacterFromActorInfo`)) (`Actor.K2_GetActorLocation` (`.Instigator` (break `GameplayEventData` EventData)))) false)))
    (:`then_1`
      (if (`self.HasMontage`)
        (`AbilityTask_PlayMontageAndWait.CreatePlayMontageAndWaitProxy` "None" (`KismetArrayLibrary.Array_Random` (`self.HitReactMontages`))
          (:`then`
            (`MeshComponent.SetScalarParameterValueOnMaterials` (`self.GetOwningComponentFromActorInfo`) "HitFxSwitch" 1.0 :!label _label)
            (if (not (`self.HasMontage`))
              (`KismetSystemLibrary.Delay` 0.2)
              (`self.K2_EndAbility`)))
          (:`OnCompleted`
            (`self.K2_EndAbility` :!label _label_2))
          (:`OnBlendOut`
            (goto _label_2))
          (:`OnInterrupted`
            (goto _label_2))
          (:`OnCancelled`
            (goto _label_2)))
        (else
          (goto _label))))
    (:`then_2`
      (`self.K2_ApplyGameplayEffectSpecToOwner` (`self.MakeOutgoingGameplayEffectSpec` "/Game/Common/_BP/Character/Enemy/Shared/GE/GE_Enemy_UnderAttack.GE_Enemy_UnderAttack_C" (`KismetMathLibrary.Conv_IntToDouble` (`self.GetAbilityLevel`)))))))

(event `self.K2_OnEndAbility`
  (params (bWasCancelled :type Boolean))
  (`MeshComponent.SetScalarParameterValueOnMaterials` (`self.GetOwningComponentFromActorInfo`) "HitFxSwitch" 0.0))