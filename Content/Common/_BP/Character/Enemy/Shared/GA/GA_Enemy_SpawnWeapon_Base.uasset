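; Base gameplay ability that spawns an enemy's weapon and attaches it to the character.
; On activation it spawns the configured weapon class with the avatar as owner and instigator, then attaches it to the owning component at a named socket.
; It registers the weapon with the enemy combat component by tag, optionally as equipped.
; The ability ends only when the spawned actor is valid.
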(event `self.K2_ActivateAbility`
  (bind _returnvalue (`self.GetAvatarActorFromActorInfo`))
  (bind _returnvalue_2 (`|SpawnActorFromClass` (`self.WeaponClass`) (`KismetMathLibrary.MakeTransform` (0.0 0.0 0.0)) "AdjustIfPossibleButAlwaysSpawn" "MultiplyWithRoot" _returnvalue (cast `Pawn` _returnvalue :!pure true)))
  (`/Engine/EditorBlueprintResources/StandardMacros.IsValid` _returnvalue_2
    (:`Is Valid`
      (`Actor.K2_AttachToComponent` _returnvalue_2 (`self.GetOwningComponentFromActorInfo`) (`self.SocketName`) "SnapToTarget" "KeepRelative" "KeepWorld" true)
      (`EnemyCombatComponent.RegisterSpawnedWeapon` (`self.GetEnemyCombatComponentFromActorInfo`) (`self.WeaponTag`) _returnvalue_2 (`self.RegisterAsEquippedWeapon`))
      (`self.K2_EndAbility`))))