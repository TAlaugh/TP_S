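; BP_Katana_Heavy is the player katana's heavy-attack actor, which applies projectile damage repeatedly while it exists.
; Tick accumulates delta time and, each time a fixed short interval elapses, resets the timer and calls HandleApplyProjectileDamage, producing periodic damage rather than per-frame hits.
; The construction script runs the parent's setup and enables actor tick; BeginPlay and overlap events are disabled placeholders.
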(event `self.ReceiveTick`
  (params (DeltaSeconds :type "Float (single-precision)"))
  (bind _output_get (set `self.ElapsedTime` (+ DeltaSeconds (`self.ElapsedTime`))))
  (if (>= _output_get 0.2)
    (set `self.ElapsedTime` 0.0)
    (`self.BP_HandleApplyProjectileDamage`)))

(fn `UserConstructionScript`
  (`parent.UserConstructionScript`)
  (`self.SetActorTickEnabled` true))