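; BP_SequenceActor is a main menu actor that triggers a fade-out sequence and a double-door opening.
; PlayFadeOut plays the SequenceFade level sequence through its sequence player.
; OpenDoor restarts a timeline whose track value is added each update as opposite world yaw deltas to DoorLeft and DoorRight, so the rotation accumulates rather than being set absolutely.
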(event `PlayFadeOut`
  (`MovieSceneSequencePlayer.Play` (`LevelSequenceActor.SequencePlayer` (`self.SequenceFade`))))

(event `OpenDoor`
  (bind (_direction _newtrack_1) (`Timeline|Timeline` :!via `PlayFromStart`)
    (:`Update`
      (`self.K2_AddActorWorldRotation` (`self.DoorLeft`) (`KismetMathLibrary.MakeRotator` 0.0 0.0 (* _newtrack_1 -1.0)) false false)
      (`self.K2_AddActorWorldRotation` (`self.DoorRight`) (`KismetMathLibrary.MakeRotator` 0.0 0.0 (* _newtrack_1 1.0)) false false))))

(fn `UserConstructionScript`)